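; Player pawn Blueprint that turns input actions into commands for its Grabber, which handles picking up and manipulating objects.
; Pressing Grab sets a flag that makes Tick call Grab every frame until Release or Reattach clears it and drops or reattaches the object.
; Other inputs forward directly to the Grabber to turn on helper mode, rotate around each axis, or reset rotation to zero.
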(event EventTick
  (params (DeltaSeconds :type Float%20%28single-precision%29))
  ;[1 1 1] Grabbing
  (if (stale Input|ActionEvents|InputActionGrab _output_get)
    (Class|Grabber|Grab (Variables|Default|GetGrabber))))

(event Input|ActionEvents|InputActionGrab
  (params (Key :type Key%20Structure))
  ;[1 1 1] Grabbing
  (:Pressed
    (bind _output_get (Variables|Default|SetIsPressed true))))

(event Input|ActionEvents|InputActionRelease
  (params (Key :type Key%20Structure))
  ;[1 1 1] Release grabbed object
  (:Pressed
    (Variables|Default|SetIsPressed false)
    (Class|Grabber|Release (Variables|Default|GetGrabber))))

(event Input|ActionEvents|InputActionRotateXAxle
  (params (Key :type Key%20Structure))
  ;[1 1 1] Rotate Grabbed Object
  (:Pressed
    (Class|Grabber|RotateXAxle (Variables|Default|GetGrabber))))

(event Input|ActionEvents|InputActionRotateToZeros
  (params (Key :type Key%20Structure))
  ;[1 1 1] Rotate Grabbed Object
  (:Pressed
    (Class|Grabber|RotatetoZeros (Variables|Default|GetGrabber))))

(event Input|ActionEvents|InputActionRotateYAxle
  (params (Key :type Key%20Structure))
  ;[1 1 1] Rotate Grabbed Object
  (:Pressed
    (Class|Grabber|RotateYAxle (Variables|Default|GetGrabber))))

(event Input|ActionEvents|InputActionRotateZAxle
  (params (Key :type Key%20Structure))
  ;[1 1 1] Rotate Grabbed Object
  (:Pressed
    (Class|Grabber|RotateZAxle (Variables|Default|GetGrabber))))

(event Input|ActionEvents|InputActionReattach
  (params (Key :type Key%20Structure))
  ;[1 1 1] Reattach
  (:Pressed
    (Variables|Default|SetIsPressed false)
    (Class|Grabber|ReattachGrabbedComponent (Variables|Default|GetGrabber))))

(event Input|ActionEvents|InputActionHelperMode
  (params (Key :type Key%20Structure))
  ;[1 1 1] Turn On/Off HelperMode
  (:Pressed
    (Class|Grabber|TurnonHelperMode (Variables|Default|GetGrabber))))

(fn ConstructionScript)